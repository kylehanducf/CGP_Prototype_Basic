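; BP_StartLevelTrigger is a box trigger that hands control to the falling player character at level start.
; BeginPlay caches player 0 as BP_CharacterFalling, and only that character's overlap starts the MoveCamera timeline.
; The timeline eases the spring arm toward a fixed -90 yaw by lerping from its current rotation each update.
; On finish, it zeroes the camera lag max distance and enables the character's input.
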(event `self.ReceiveBeginPlay`
  (bind _asbp_character_falling (cast `/Game/Blueprints/Character/BP_CharacterFalling` (`GameplayStatics.GetPlayerCharacter` 0)))
  (set `self.Character` _asbp_character_falling))

(event `self.Box.OnComponentBeginOverlap`
  (params (OverlappedComponent :type "PrimitiveComponent Object Reference") (OtherActor :type "Actor Object Reference") (OtherComp :type "PrimitiveComponent Object Reference") (OtherBodyIndex :type Integer) (bFromSweep :type Boolean) (SweepResult :type "HitResult Structure (by ref)"))
  (if (== OtherActor (`self.Character`))
    (bind (_direction _alpha) (`Timeline|MoveCamera`)
      (:`Update`
        (`SceneComponent.K2_SetRelativeRotation` (`/Game/Blueprints/Character/BP_CharacterFalling.SpringArm` (`self.Character`)) (`KismetMathLibrary.RLerp` (`SceneComponent.RelativeRotation` (`/Game/Blueprints/Character/BP_CharacterFalling.SpringArm` (`self.Character`))) (struct :`Pitch` -90.0) _alpha true) false false))
      (:`Finished`
        (set `SpringArmComponent.CameraLagMaxDistance` 0.0 (`/Game/Blueprints/Character/BP_CharacterFalling.SpringArm` (`self.Character`)))
        (`self.EnableInput` (`self.Character`) null)))))

(fn `UserConstructionScript`)