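; BP_Crusher is an obstacle with two crusher arms that slam back and forth between start and end markers.
; On BeginPlay it takes a random yaw and starts the T_Slam timeline, which lerps both arms' world locations without sweeping.
; When the timeline finishes, it waits a random few seconds, then uses the Loop flag to alternate between reverse and forward playback indefinitely.
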(event `Play`
  (bind (_direction _alpha) (`Timeline|T_Slam` :!label _label)
    (:`Update`
      (`SceneComponent.K2_SetWorldLocation` (`self.CrusherArmA`) (`KismetMathLibrary.VLerp` (`SceneComponent.K2_GetComponentLocation` (`self.CrusherAEnd`)) (`SceneComponent.K2_GetComponentLocation` (`self.CrusherAStart`)) _alpha) false false)
      (`SceneComponent.K2_SetWorldLocation` (`self.CrusherArmB`) (`KismetMathLibrary.VLerp` (`SceneComponent.K2_GetComponentLocation` (`self.CrusherBEnd`)) (`SceneComponent.K2_GetComponentLocation` (`self.CrusherBStart`)) _alpha) false false))
    (:`Finished`
      (`KismetSystemLibrary.Delay` (`KismetMathLibrary.RandomFloatInRange` 1.0 5.0))
      (if (`self.Loop`)
        (set `self.Loop` false)
        (`self.Reverse`)
        (else
          (set `self.Loop` true)
          (`self.Play`))))))

(event `self.ReceiveBeginPlay`
  (`self.K2_SetActorRotation` (`KismetMathLibrary.MakeRotator` 0.0 0.0 (`KismetMathLibrary.RandomFloatInRange` 0.0 360.0)))
  (goto _label :!via `PlayFromStart`))

(event `Reverse`
  (goto _label :!via `Reverse`))

(fn `UserConstructionScript`)