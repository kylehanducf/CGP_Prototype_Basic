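; Obstacle spawner that raises a bucket on an elevator platform and releases BP_LavaBucket actors in a repeating cycle.
; An oscillating timeline moves the platform between spawn and elevate points, pausing randomly after each run.
; A Loop flag alternates the cycle: one pass opens the doors, spawns a bucket above the elevate point, hides the display bucket and reverses.
; The other pass shows the display bucket again and replays the lift.
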(event `Play`
  (bind (_direction _alpha) (`Timeline|T_Occilate` :!label _label)
    (:`Update`
      (`SceneComponent.K2_SetWorldLocation` (`self.Platform`) (`KismetMathLibrary.VLerp` (`SceneComponent.K2_GetComponentLocation` (`self.SpawnPoint`)) (`SceneComponent.K2_GetComponentLocation` (`self.ElevatePoint`)) _alpha) false false))
    (:`Finished`
      (`KismetSystemLibrary.Delay` (`KismetMathLibrary.RandomFloatInRange` 1.0 3.0))
      (if (`self.Loop`)
        (set `self.Loop` false)
        (`self.DoorOpen`)
        (`KismetSystemLibrary.Delay` 1.0)
        (`self.Spawn`)
        (`SceneComponent.SetVisibility` (`self.Bucket`) false false)
        (`KismetSystemLibrary.Delay` 1.0)
        (`self.Reverse`)
        (`self.DoorClose`)
        (else
          (set `self.Loop` true)
          (`SceneComponent.SetVisibility` (`self.Bucket`) true false)
          (`self.Play`))))))

(event `self.ReceiveBeginPlay`
  (goto _label :!via `PlayFromStart`))

(event `Reverse`
  (goto _label :!via `Reverse`))

(event `Spawn`
  (bind (_returnvalue_x _returnvalue_y _returnvalue_z) (`KismetMathLibrary.BreakVector` (`SceneComponent.K2_GetComponentLocation` (`self.ElevatePoint`))))
  (`|SpawnActorFromClass` "/Game/Blueprints/Obstacles/Obstacles/LavaBucket/BP_LavaBucket.BP_LavaBucket_C" (`KismetMathLibrary.Conv_VectorToTransform` (`KismetMathLibrary.MakeVector` _returnvalue_x _returnvalue_y (+ _returnvalue_z 150.0))) "Undefined" "OverrideRootScale" null null))

(event `DoorOpen`
  (bind (_direction _alpha) (`Timeline|T_DoorMovement` :!via `PlayFromStart` :!label _label_2)
    (:`Update`
      (`SceneComponent.K2_SetWorldLocation` (`self.DoorLeft`) (`KismetMathLibrary.VLerp` (`SceneComponent.K2_GetComponentLocation` (`self.LeftDoorClosed`)) (`SceneComponent.K2_GetComponentLocation` (`self.LeftDoorOpen`)) _alpha) false false)
      (`SceneComponent.K2_SetWorldLocation` (`self.DoorRight`) (`KismetMathLibrary.VLerp` (`SceneComponent.K2_GetComponentLocation` (`self.RightDoorClosed`)) (`SceneComponent.K2_GetComponentLocation` (`self.RightDoorOpen`)) _alpha) false false))))

(event `DoorClose`
  (goto _label_2 :!via `ReverseFromEnd`))

(fn `UserConstructionScript`)