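; BP_Propeller is an obstacle actor that spins continuously around its yaw axis.
; On BeginPlay it picks a random SpinSpeed, which acts as a divisor, so larger values spin slower.
; Each Tick it lerps from the current rotation toward 90 degrees further in yaw by DeltaSeconds over SpinSpeed, giving a steady frame-rate-scaled rotation.
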(event `self.ReceiveBeginPlay`
  (set `self.SpinSpeed` (`KismetMathLibrary.RandomFloatInRange` 1.0 2.0)))

(event `self.ReceiveTick`
  (params (DeltaSeconds :type "Float (single-precision)"))
  (bind _returnvalue (`self.K2_GetActorRotation`))
  (`self.K2_SetActorRotation` (`KismetMathLibrary.RLerp` _returnvalue (`KismetMathLibrary.MakeRotator` (.roll _returnvalue) (.pitch _returnvalue) (+ (.yaw _returnvalue) 90.0)) (/ DeltaSeconds (`self.SpinSpeed`)))))

(fn `UserConstructionScript`)