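; BP_LaserCutter is a spinning laser obstacle that damages the player character on contact.
; It starts at a random yaw with tinted Niagara effects, then rotates each Tick at a randomly varying speed.
; DrawLaser sphere-traces forward every frame, damaging the player if hit and placing the flickering beam's end, impact and sparks at the hit point.
; Overlapping MainCollision also damages the player.
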(event `self.ReceiveBeginPlay`
  (`FXSystemComponent.SetColorParameter` (`self.NiagaraLaser`) "Color" (`self.LaserColor`))
  (`FXSystemComponent.SetColorParameter` (`self.NiagaraLaserImpact`) "Color" (`self.LaserColor`))
  (`FXSystemComponent.SetColorParameter` (`self.NiagaraLaserSparks`) "Color" (`self.SparksColor`))
  (`SceneComponent.SetVisibility` (`self.NiagaraLaser`) true false)
  (`self.K2_SetActorRotation` (`KismetMathLibrary.MakeRotator` 0.0 0.0 (`KismetMathLibrary.RandomFloatInRange` 0.0 360.0)))
  (bind _asbp_character_falling (cast `/Game/Blueprints/Character/BP_CharacterFalling` (`GameplayStatics.GetPlayerCharacter` 0)))
  (set `self.Character` _asbp_character_falling))

(event `self.ReceiveTick`
  (params (DeltaSeconds :type "Float (single-precision)"))
  (bind (_returnvalue_roll _returnvalue_pitch _returnvalue_yaw) (`KismetMathLibrary.BreakRotator` (`self.K2_GetActorRotation`)))
  (`self.DrawLaser`)
  (`self.K2_SetActorRotation` (`KismetMathLibrary.RLerp` (`KismetMathLibrary.MakeRotator` _returnvalue_roll _returnvalue_pitch _returnvalue_yaw) (`KismetMathLibrary.MakeRotator` _returnvalue_roll _returnvalue_pitch (+ _returnvalue_yaw 90.0)) (/ DeltaSeconds (`KismetMathLibrary.RandomFloatInRange` 0.5 5.0)))))

(event `self.MainCollision.OnComponentBeginOverlap`
  (params (OverlappedComponent :type "PrimitiveComponent Object Reference") (OtherActor :type "Actor Object Reference") (OtherComp :type "PrimitiveComponent Object Reference") (OtherBodyIndex :type Integer) (bFromSweep :type Boolean) (SweepResult :type "HitResult Structure (by ref)"))
  (if (== OtherActor (`self.Character`))
    (`GameplayStatics.ApplyDamage` (`self.Character`) (`self.BaseDamage`))))

(fn `DrawLaser`
  (bind _returnvalue (`SceneComponent.K2_GetComponentLocation` (`self.NiagaraLaser`)))
  (set `self.TraceStart` _returnvalue)
  (set `self.TraceEnd` (+ _returnvalue (* (`self.GetActorForwardVector`) (`self.LaserDistance`))))
  (bind (_outhit _returnvalue_2) (`KismetSystemLibrary.SphereTraceSingle` (`self.TraceStart`) (`self.TraceEnd`) 20.0 "TraceTypeQuery1"))
  (set `self.IsLaserHitting` _returnvalue_2)
  (bind (_bblockinghit _binitialoverlap _time _distance _location _impactpoint _normal _impactnormal _physmat _hitactor) (`GameplayStatics.BreakHitResult` _outhit))
  (set `self.LaserHitLocation` _impactpoint)
  (`|ExecutionSequence`
    (:`then_0`
      (if (== _hitactor (`self.Character`))
        (`GameplayStatics.ApplyDamage` (`self.Character`) (`self.BaseDamage`))))
    (:`then_1`
      (`FXSystemComponent.SetVectorParameter` (`self.NiagaraLaser`) "LaserEndPoint" (select `bool` (`self.IsLaserHitting`) :`false` (`self.TraceEnd`) :`true` (`self.LaserHitLocation`)))
      (`SceneComponent.SetVisibility` (`self.NiagaraLaserImpact`) (`self.IsLaserHitting`) false)
      (`SceneComponent.SetVisibility` (`self.NiagaraLaserSparks`) (`self.IsLaserHitting`) false)
      (`SceneComponent.K2_SetWorldLocation` (`self.NiagaraLaserImpact`) (`self.LaserHitLocation`) false false)
      (`SceneComponent.K2_SetWorldLocation` (`self.NiagaraLaserSparks`) (`self.LaserHitLocation`) false false)
      (`FXSystemComponent.SetFloatParameter` (`self.NiagaraLaser`) "BeamWidth" (`KismetMathLibrary.RandomFloatInRange` 15.0 50.0)))))

(fn `UserConstructionScript`)