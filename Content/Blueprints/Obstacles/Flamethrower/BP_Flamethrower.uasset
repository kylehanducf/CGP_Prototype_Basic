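; BP_Flamethrower is an obstacle that damages the player's BP_CharacterFalling with a flame and on contact with its barrel.
; It caches the character and picks a random yaw at BeginPlay.
; Each Tick, a sphere trace from the Niagara flame along the actor's forward vector applies damage whenever it hits the character, so damage is per frame.
; Spin and laser-style beam visual logic exist but are disconnected.
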(event `self.ReceiveBeginPlay`
  (bind _asbp_character_falling (cast `/Game/Blueprints/Character/BP_CharacterFalling` (`GameplayStatics.GetPlayerCharacter` 0)))
  (set `self.Character` _asbp_character_falling)
  (`self.K2_SetActorRotation` (`KismetMathLibrary.MakeRotator` 0.0 0.0 (`KismetMathLibrary.RandomFloatInRange` 0.0 360.0))))

(event `self.ReceiveTick`
  (params (DeltaSeconds :type "Float (single-precision)"))
  (`self.DrawFlamethrower`))

(event `self.BarrelCollision.OnComponentBeginOverlap`
  (params (OverlappedComponent :type "PrimitiveComponent Object Reference") (OtherActor :type "Actor Object Reference") (OtherComp :type "PrimitiveComponent Object Reference") (OtherBodyIndex :type Integer) (bFromSweep :type Boolean) (SweepResult :type "HitResult Structure (by ref)"))
  (if (== OtherActor (`self.Character`))
    (`GameplayStatics.ApplyDamage` (`self.Character`) (`self.BaseDamage`))))

(fn `DrawFlamethrower`
  (bind _returnvalue (`SceneComponent.K2_GetComponentLocation` (`self.NiagaraFlame`)))
  (set `self.TraceStart` _returnvalue)
  (set `self.TraceEnd` (+ _returnvalue (* (`self.GetActorForwardVector`) (`self.FlameDistance`))))
  (bind (_outhit _returnvalue_2) (`KismetSystemLibrary.SphereTraceSingle` (`self.TraceStart`) (`self.TraceEnd`) 30.0 "TraceTypeQuery1"))
  (set `self.IsLaserHitting` _returnvalue_2)
  (if (== (`.HitActor` (`GameplayStatics.BreakHitResult` _outhit)) (`self.Character`))
    (`GameplayStatics.ApplyDamage` (`self.Character`) (`self.BaseDamage`))))

(fn `UserConstructionScript`)