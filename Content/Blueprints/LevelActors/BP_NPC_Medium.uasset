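; Level NPC that selects the medium difficulty when the player interacts with it inside its trigger box.
; Box overlap with the player character enables interaction and shows two objective components, hiding them on exit.
; Tick polls the character's interacting flag, then writes difficulty, collectable and life targets to the GameInstance, keeping completion states.
; Its DoOnce resets immediately, so the write repeats every frame while interacting.
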(event `self.ReceiveBeginPlay`
  (bind _asbp_character (cast `/Game/Blueprints/Character/BP_Character` (`GameplayStatics.GetPlayerCharacter` 0)))
  (set `self.Character` _asbp_character)
  (bind _asgi_game_instance (cast `/Game/GameFiles/GI_GameInstance` (`GameplayStatics.GetGameInstance`)))
  (set `self.GameInstance` _asgi_game_instance))

(event `self.ReceiveTick`
  (params (DeltaSeconds :type "Float (single-precision)"))
  (if (`self.CanInteract`)
    (if (`/Game/Blueprints/Character/BP_Character.IsInteracting` (`self.Character`))
      (`/Engine/EditorBlueprintResources/StandardMacros.DoOnce` false :!label _label
        (:`Completed`
          (`/Game/GameFiles/GI_GameInstance.SetDifficulty` (`self.GameInstance`) 1)
          (bind _objective3complete (`/Game/GameFiles/GI_GameInstance.GetObjective3` (`self.GameInstance`)))
          (`/Game/GameFiles/GI_GameInstance.SetObjective3` (`self.GameInstance`) _objective3complete 12)
          (bind _objective4complete (`/Game/GameFiles/GI_GameInstance.GetObjective4` (`self.GameInstance`)))
          (`/Game/GameFiles/GI_GameInstance.SetObjective4` (`self.GameInstance`) _objective4complete 2)
          (goto _label :!via `Reset`))))))

(event `self.Box.OnComponentBeginOverlap`
  (params (OverlappedComponent :type "PrimitiveComponent Object Reference") (OtherActor :type "Actor Object Reference") (OtherComp :type "PrimitiveComponent Object Reference") (OtherBodyIndex :type Integer) (bFromSweep :type Boolean) (SweepResult :type "HitResult Structure (by ref)"))
  (if (== OtherActor (`self.Character`))
    (set `self.CanInteract` true)
    (`SceneComponent.SetVisibility` (`self.Objective1`) true false)
    (`SceneComponent.SetVisibility` (`self.Objective2`) true false)))

(event `self.Box.OnComponentEndOverlap`
  (params (OverlappedComponent :type "PrimitiveComponent Object Reference") (OtherActor :type "Actor Object Reference") (OtherComp :type "PrimitiveComponent Object Reference") (OtherBodyIndex :type Integer))
  (if (== OtherActor (`self.Character`))
    (set `self.CanInteract` false)
    (`SceneComponent.SetVisibility` (`self.Objective1`) false false)
    (`SceneComponent.SetVisibility` (`self.Objective2`) false false)))

(fn `UserConstructionScript`)