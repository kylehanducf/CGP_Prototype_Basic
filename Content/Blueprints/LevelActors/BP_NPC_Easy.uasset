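; BP_NPC_Easy is an NPC actor that sets the game to Easy difficulty when the player interacts with it.
; Overlapping its Box enables interaction and shows the Objective component.
; Tick polls the character's IsInteracting flag, then sets difficulty and both objectives' collectable and lives values on the GameInstance, keeping completion states.
; Its DoOnce resets immediately, so these writes repeat while interaction is held.
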(event `self.ReceiveBeginPlay`
  (bind _asbp_character (cast `/Game/Blueprints/Character/BP_Character` (`GameplayStatics.GetPlayerCharacter` 0)))
  (set `self.Character` _asbp_character)
  (bind _asgi_game_instance (cast `/Game/GameFiles/GI_GameInstance` (`GameplayStatics.GetGameInstance`)))
  (set `self.GameInstance` _asgi_game_instance))

(event `self.ReceiveTick`
  (params (DeltaSeconds :type "Float (single-precision)"))
  (if (`self.CanInteract`)
    (if (`/Game/Blueprints/Character/BP_Character.IsInteracting` (`self.Character`))
      (`/Engine/EditorBlueprintResources/StandardMacros.DoOnce` false :!label _label
        (:`Completed`
          (`/Game/GameFiles/GI_GameInstance.SetDifficulty` (`self.GameInstance`) 0)
          (bind _objective1complete (`/Game/GameFiles/GI_GameInstance.GetObjective1` (`self.GameInstance`)))
          (`/Game/GameFiles/GI_GameInstance.SetObjective1` (`self.GameInstance`) _objective1complete 10)
          (bind _objective2complete (`/Game/GameFiles/GI_GameInstance.GetObjective2` (`self.GameInstance`)))
          (`/Game/GameFiles/GI_GameInstance.SetObjective2` (`self.GameInstance`) _objective2complete 0)
          (goto _label :!via `Reset`))))))

(event `self.Box.OnComponentBeginOverlap`
  (params (OverlappedComponent :type "PrimitiveComponent Object Reference") (OtherActor :type "Actor Object Reference") (OtherComp :type "PrimitiveComponent Object Reference") (OtherBodyIndex :type Integer) (bFromSweep :type Boolean) (SweepResult :type "HitResult Structure (by ref)"))
  (if (== OtherActor (`self.Character`))
    (set `self.CanInteract` true)
    (`SceneComponent.SetVisibility` (`self.Objective`) true false)))

(event `self.Box.OnComponentEndOverlap`
  (params (OverlappedComponent :type "PrimitiveComponent Object Reference") (OtherActor :type "Actor Object Reference") (OtherComp :type "PrimitiveComponent Object Reference") (OtherBodyIndex :type Integer))
  (if (== OtherActor (`self.Character`))
    (set `self.CanInteract` false)
    (`SceneComponent.SetVisibility` (`self.Objective`) false false)))

(fn `UserConstructionScript`)