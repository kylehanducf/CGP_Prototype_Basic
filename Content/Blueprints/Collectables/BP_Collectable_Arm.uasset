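; Arm collectable that adds one to the falling player character's CurrentScrap when picked up.
; On BeginPlay it binds to the pickup event, which stops rotation and destroys the sphere component when fired.
; The PickupAnimation timeline then updates mesh location and scale through helper graphs containing lerps toward the player and a small size.
; When the timeline finishes, it increments the scrap count and destroys the actor.
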(event `self.ReceiveBeginPlay`
  (`parent.ReceiveBeginPlay`)
  (add `self.Pickup` (delegate `PickupGrabbed`)))

(event `PickupGrabbed`
  (bind _asbp_character_falling (cast `/Game/Blueprints/Character/BP_CharacterFalling` (`GameplayStatics.GetPlayerCharacter` 0)))
  (set `self.PlayerCharacter` _asbp_character_falling)
  (`TimelineComponent.Stop` (`self.Rotating`))
  (`ActorComponent.K2_DestroyComponent` (`self.Sphere`))
  (bind (_direction _alpha) (`Timeline|PickupAnimation` :!via `PlayFromStart`)
    (:`Update`
      (bind _output_get (set `self.Alpha` _alpha))
      (`SceneComponent.K2_SetWorldLocation` (`self.StaticMesh`) (`self.GetMeshLocation` _output_get) false false)
      (`SceneComponent.SetRelativeScale3D` (`self.StaticMesh`) (`self.GetMeshScale`)))
    (:`Finished`
      (bind _result (`/Engine/EditorBlueprintResources/StandardMacros.IncrementInt` (`/Game/Blueprints/Character/BP_CharacterFalling.CurrentScrap` (`self.PlayerCharacter`)))
        (:`  `
          (set `/Game/Blueprints/Character/BP_CharacterFalling.CurrentScrap` _result (`self.PlayerCharacter`))
          (`self.K2_DestroyActor`))))))

(fn `UserConstructionScript`
  (`parent.UserConstructionScript`))