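; Base collectable actor that flies to the falling player character and is destroyed on pickup.
; On BeginPlay it caches the BP_CharacterFalling player and sizes its overlap sphere from the PickupRadius variable.
; When the player overlaps the sphere, a timeline lerps the actor from its current location toward the character's live location each update, then destroys it when finished.
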(event `self.ReceiveBeginPlay`
  (bind _asbp_character_falling (cast `/Game/Blueprints/Character/BP_CharacterFalling` (`GameplayStatics.GetPlayerCharacter` 0)))
  (set `self.Character` _asbp_character_falling)
  (`SphereComponent.SetSphereRadius` (`self.Sphere`) (`self.PickupRadius`) true))

(event `self.Sphere.OnComponentBeginOverlap`
  (params (OverlappedComponent :type "PrimitiveComponent Object Reference") (OtherActor :type "Actor Object Reference") (OtherComp :type "PrimitiveComponent Object Reference") (OtherBodyIndex :type Integer) (bFromSweep :type Boolean) (SweepResult :type "HitResult Structure (by ref)"))
  (if (== OtherActor (`self.Character`))
    (bind (_direction _distance_normalised_) (`Timeline|T_Attraction` :!via `PlayFromStart`)
      (:`Update`
        (`self.K2_SetActorLocation` (`KismetMathLibrary.VLerp` (`self.K2_GetActorLocation`) (`self.K2_GetActorLocation` (`self.Character`)) _distance_normalised_)))
      (:`Finished`
        (`self.K2_DestroyActor`)))))

(fn `UserConstructionScript`)