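; End-of-level trigger volume for the falling game that plays a landing sequence when the player's BP_CharacterFalling overlaps its box.
; It shuts the character down, disables input, zeroes gravity and velocity, and blends the view to the BP_EndCamera actor.
; With both boosters active, a timeline lerps the character between fixed world positions on the centre axis, overriding its entry location.
; When the timeline finishes, boosters switch off and the cursor and LevelComplete_Widget appear.
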(event `self.ReceiveBeginPlay`
  (bind _asbp_character_falling (cast `/Game/Blueprints/Character/BP_CharacterFalling` (`GameplayStatics.GetPlayerCharacter` 0)))
  (set `self.Character` _asbp_character_falling))

(event `self.Box.OnComponentBeginOverlap`
  (params (OverlappedComponent :type "PrimitiveComponent Object Reference") (OtherActor :type "Actor Object Reference") (OtherComp :type "PrimitiveComponent Object Reference") (OtherBodyIndex :type Integer) (bFromSweep :type Boolean) (SweepResult :type "HitResult Structure (by ref)"))
  (bind _character (`self.Character`))
  (bind _character_2 (`self.Character`))
  (bind _character_3 (`self.Character`))
  (bind _charactermovement (`Character.CharacterMovement` _character))
  (if (== OtherActor (`self.Character`))
    (`/Game/Blueprints/Character/BP_CharacterFalling.TurnEverythingOff` (`self.Character`))
    (`self.DisableInput` _character null)
    (set `CharacterMovementComponent.GravityScale` 0.0 _charactermovement)
    (set `MovementComponent.Velocity` (0.0 0.0 0.0) _charactermovement)
    (bind _returnvalue (`GameplayStatics.GetActorOfClass` "/Game/Blueprints/BP_EndCamera.BP_EndCamera_C"))
    (`PlayerController.SetViewTargetWithBlend` (`GameplayStatics.GetPlayerController` 0) _returnvalue 2.0 "VTBlend_Linear" 0.0 false)
    (`ActorComponent.SetActive` (`/Game/Blueprints/Character/BP_CharacterFalling.BoosterLeft` _character_3) true false)
    (`ActorComponent.SetActive` (`/Game/Blueprints/Character/BP_CharacterFalling.BoosterRight` _character_3) true false)
    (bind (_direction _alpha) (`Timeline|T_CenterCharacter`)
      (:`Update`
        (`self.K2_SetActorLocation` (`self.Character`) (`KismetMathLibrary.VLerp` (0.0 0.0 -102000.0) (0.0 0.0 -106950.0) _alpha) false false))
      (:`Finished`
        (`ActorComponent.SetActive` (`/Game/Blueprints/Character/BP_CharacterFalling.BoosterLeft` _character_2) false false)
        (`ActorComponent.SetActive` (`/Game/Blueprints/Character/BP_CharacterFalling.BoosterRight` _character_2) false false)
        (set `PlayerController.bShowMouseCursor` true (`GameplayStatics.GetPlayerController` 0))
        (bind _returnvalue_2 (`|CreateWidget` "/Game/Blueprints/UI/Widgets/LevelComplete_Widget.LevelComplete_Widget_C"))
        (`UserWidget.AddToViewport` _returnvalue_2 0)))))

(fn `UserConstructionScript`)