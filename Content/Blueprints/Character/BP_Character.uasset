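; BP_Character is a player-controlled Character with two-axis movement and a held interact input.
; It disables player input on BeginPlay.
; MoveUp and MoveRight move it along fixed world X and Y axes, while Interact sets IsInteracting true on press and false on release.
; A GetCharacterDirection helper derives forward and right vectors from control yaw, but movement does not use it.
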(event `self.ReceiveBeginPlay`
  (`self.DisableInput` (`GameplayStatics.GetPlayerController` 0)))

(event `InputAxis|MoveUp`
  (params (AxisValue :type "Float (single-precision)"))
  (`self.AddMovementInput` (1.0 0.0 0.0) AxisValue))

(event `InputAxis|MoveRight`
  (params (AxisValue :type "Float (single-precision)"))
  (`self.AddMovementInput` (0.0 1.0 0.0) AxisValue))

(event `InputAction|Interact`
  (params (Key :type "Key Structure"))
  (:`Pressed`
    (set `self.IsInteracting` true))
  (:`Released`
    (set `self.IsInteracting` false)))

(fn `GetCharacterDirection`
  (returns (ForwardVector :type "Vector Structure") (RightVector :type "Vector Structure"))
  (bind _returnvalue (`KismetMathLibrary.MakeRotator` 0.0 0.0 (.yaw (`self.GetControlRotation`))))
  (return (`KismetMathLibrary.GetForwardVector` _returnvalue) (`KismetMathLibrary.GetRightVector` _returnvalue)))

(fn `UserConstructionScript`)